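; BP_MainLevel is the moving level actor for the Sticky Situation minigame, scrolling steadily along its local negative Y axis.
; On start it shuffles an item pool, spawns one item at a random point in each of four boxes, attaches them, and boosts speed after a delay.
; The game mode's reset event, gated by HasReset, restores position and speed, destroys spawned items and reruns that setup.
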(event Custom|MinigameReset
  (bind _allspawnedactors (Variables|Default|GetAllSpawnedActors))
  (if (Variables|Default|GetHasReset)
    (Transformation|SetActorLocation (Variables|Default|GetStartLocation) false false)
    (if (Variables|Default|GetIsFaster)
      (Variables|Default|SetInitialSpeed (+ (Variables|Default|GetInitialSpeed) -5e+02))
      (Variables|Default|SetIsFaster false))
    (for _array_element _allspawnedactors
      (Actor|DestroyActor _array_element))
    (Utilities|Array|Clear _allspawnedactors)
    (Variables|Default|SetItemIndex 0)
    (Variables|Default|SetHasReset true)
    (Utilities|Array|Shuffle (Variables|Default|GetItemsPool))
    (CallFunction|SpawnIteminBox (Variables|Default|GetSpawnBox1))
    (CallFunction|SpawnIteminBox (Variables|Default|GetSpawnBox2))
    (CallFunction|SpawnIteminBox (Variables|Default|GetSpawnBox3))
    (CallFunction|SpawnIteminBox (Variables|Default|GetSpawnBox4))
    (Utilities|FlowControl|Delay 19.0)
    (Variables|Default|SetInitialSpeed (+ (Variables|Default|GetInitialSpeed) 5e+02))
    (Variables|Default|SetIsFaster true)))

(event EventTick
  (params (DeltaSeconds :type Float%20%28single-precision%29))
  (Transformation|AddActorLocalOffset (Math|Vector|MakeVector 0.0 (* (* (Variables|Default|GetInitialSpeed) DeltaSeconds) -1.0) 0.0) false false))

(event EventBeginPlay
  (bind _asbp_sticky_situation_game_mode (Utilities|Casting|CastToBP_StickySituationGameMode (Game|GetGameMode))
    (:then
      (EventDispatchers|BindEventtoOnMinigameResetEvent _asbp_sticky_situation_game_mode (delegate Custom|MinigameReset)))
    (:CastFailed
      _))
  (Variables|Default|SetStartLocation (Transformation|GetActorLocation))
  (Utilities|Array|Shuffle (Variables|Default|GetItemsPool))
  (CallFunction|SpawnIteminBox (Variables|Default|GetSpawnBox1))
  (CallFunction|SpawnIteminBox (Variables|Default|GetSpawnBox2))
  (CallFunction|SpawnIteminBox (Variables|Default|GetSpawnBox3))
  (CallFunction|SpawnIteminBox (Variables|Default|GetSpawnBox4))
  (Utilities|FlowControl|Delay 19.0)
  (Variables|Default|SetInitialSpeed (+ (Variables|Default|GetInitialSpeed) 5e+02))
  (Variables|Default|SetIsFaster true))

(fn ConstructionScript)

(fn SpawnIteminBox
  (params (CurrentBox :type Box%20Component%20Object%20Reference))
  (bind _returnvalue (Game|SpawnActorfromClass (Utilities|Array|Get(acopy) (Variables|Default|GetItemsPool) (Variables|Default|GetItemIndex)) (Math|Transform|MakeTransform (Math|Random|RandomPointinBoundingBox (Transformation|GetWorldLocation CurrentBox) (Variables|/Script/Engine.BoxComponent|GetBoxExtent CurrentBox)) "0, 0, 0" "1.000000,1.000000,1.000000") "Undefined" "MultiplyWithRoot" 0 0))
  (Transformation|AttachActorToActor _returnvalue self "None" "KeepWorld" "KeepWorld" "KeepWorld" true)
  (Variables|Default|SetItemIndex (+ (Variables|Default|GetItemIndex) 1))
  (Utilities|Array|Add (Variables|Default|GetAllSpawnedActors) _returnvalue))