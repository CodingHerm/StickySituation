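; Player pawn for the Sticky Situation minigame that moves along world X and collects orbs for points.
; Button1 or AnalogFlex destroys overlapping BP_Orb actors, adding a point each to the player's counter and printing the total.
; A timeline scrubs the skeletal mesh's animation back and forth continuously.
; Each tick, a downward line trace feeds an interpolated Z position so the pawn follows the surface below.
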(event Input|EnhancedActionEvents|EnhancedInputActionIA_AnalogFlex
  (params (ActionValue :type Float%20%28double-precision%29) (ElapsedSeconds :type Float%20%28double-precision%29) (TriggeredSeconds :type Float%20%28double-precision%29) (InputAction :type Input%20Action%20Object%20Reference :default "/LimbitlessBluetoothPlugin/InputActions/IA_AnalogFlex.IA_AnalogFlex"))
  (bind _playernumber (Variables|Default|GetPlayerNumber))
  (bind _minigame (Variables|Default|GetMinigame))
  (bind _returnvalue (Class|MinigameBase|GetPointCounter _minigame))
  (for _array_element (Collision|GetOverlappingActors "/Game/BP_Orb.BP_Orb_C" :!class /Script/Engine.Actor)
    (Actor|DestroyActor _array_element)
    (Class|BasePointCounter|AddPoints _returnvalue _playernumber 1)
    (Development|PrintString (Utilities|String|ToString(Integer) (Class|BasePointCounter|GetPointsbyPlayer _returnvalue _playernumber)))))

(event Input|EnhancedActionEvents|EnhancedInputActionIA_Movement
  (params (ActionValue :type Vector%202D%20Structure) (ElapsedSeconds :type Float%20%28double-precision%29) (TriggeredSeconds :type Float%20%28double-precision%29) (InputAction :type Input%20Action%20Object%20Reference :default "/MinigameCore/Input/IA_Movement.IA_Movement"))
  (Class|PawnMovementComponent|AddInputVector (Variables|Default|GetFloatingPawnMovement) (Math|Vector|MakeVector (* (* (.x ActionValue) -1.0) (Variables|Default|GetPlayerSpeed)) 0.0 0.0) false))

(event Input|EnhancedActionEvents|EnhancedInputActionIA_Button1
  (params (ActionValue :type Boolean) (ElapsedSeconds :type Float%20%28double-precision%29) (TriggeredSeconds :type Float%20%28double-precision%29) (InputAction :type Input%20Action%20Object%20Reference :default "/MinigameCore/Input/IA_Button1.IA_Button1"))
  (bind _playernumber (Variables|Default|GetPlayerNumber))
  (bind _minigame (Variables|Default|GetMinigame))
  (bind _returnvalue (Class|MinigameBase|GetPointCounter _minigame))
  (for _array_element (Collision|GetOverlappingActors "/Game/BP_Orb.BP_Orb_C" :!class /Script/Engine.Actor)
    (Actor|DestroyActor _array_element)
    (Class|BasePointCounter|AddPoints _returnvalue _playernumber 1)
    (Development|PrintString (Utilities|String|ToString(Integer) (Class|BasePointCounter|GetPointsbyPlayer _returnvalue _playernumber)))))

(event EventBeginPlay
  (bind _newtrack_0 (Timeline|PingPongTimeline PlayFromStart)
    (:Update
      (Components|Animation|SetPosition (Variables|Default|GetSkeletalMesh) _newtrack_0 true))
    (:Finished
      (Utilities|FlowControl|FlipFlop
        (:A
          (Timeline|PingPongTimeline Reverse))
        (:B
          (Timeline|PingPongTimeline Play))))))

(event EventTick
  (params (DeltaSeconds :type Float%20%28single-precision%29))
  (bind _returnvalue (Transformation|GetActorLocation))
  (bind (_x _y _z) (Math|Vector|BreakVector _returnvalue))
  (bind _outhit (Collision|LineTraceByChannel (+ (Transformation|GetActorLocation) "0.000000,0.000000,100.000000") (+ (Transformation|GetActorLocation) "0.000000,0.000000,-500.000000") "TraceTypeQuery1" false 0 "None"))
  (Transformation|SetActorLocation (Math|Vector|MakeVector _x _y (Math|Interpolation|FInterpTo _z (.Z (Math|Vector|BreakVector (.ImpactPoint (Collision|BreakHitResult _outhit)))) (Utilities|Time|GetWorldDeltaSeconds) 1e+01)) false false))

(fn ConstructionScript)